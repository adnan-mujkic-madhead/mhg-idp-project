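; BP_MinimapCameraActor is an actor that keeps character positions on the minimap widget up to date.
; On BeginPlay it collects every LiraCharacter in the level once and caches MainUI from BP_LiraPlayerController.
; Each Tick, while MainUI is valid, it passes every cached character to WBPMinimap's UpdateWidgetPosition.
; Characters spawned after BeginPlay are not added to the list by this Blueprint.
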(event EventBeginPlay
  (bind _outactors (Actor|GetAllActorsOfClass "/Script/Lira.LiraCharacter"))
  (for _array_element _outactors
    (Utilities|Array|AddUnique (Variables|Default|GetLira%20Characters) _array_element))
  (bind _asbp_lira_player_controller (Utilities|Casting|CastToBP_LiraPlayerController (Game|GetPlayerController 0)))
  (Variables|Default|SetMain%20UI (Variables|/Game/ThirdPerson/Blueprints/BP_LiraPlayerController.BP_LiraPlayerController_C|GetMain%20UI _asbp_lira_player_controller)))

(event EventTick
  (params (DeltaSeconds :type Float%20%28single-precision%29))
  (bind _main_ui (Variables|Default|GetMain%20UI)
    (:then
      (for _array_element (Variables|Default|GetLira%20Characters)
        (Default|UpdateWidgetPosition (Variables|/Game/UI/WBP_MainUI.WBP_MainUI_C|GetWBP_Minimap _main_ui) _array_element)))
    (:else)))

(fn ConstructionScript)